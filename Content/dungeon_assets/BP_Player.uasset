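; Player Blueprint that tracks Gold and Round and resolves the outcome of each level.
; BeginPlay binds to an end-of-level dispatcher; EndOfLevel counts any surviving BP_MasterU actor tagged "Friendly" as a victory, then unbinds all dispatcher events.
; Victory adds each survivor's Cost to Gold and increments Round, while defeat only prints a message because its handler is empty.
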(event EventBeginPlay
  (EventDispatchers|BindEventtoEndOfLevelDispatcher (EventDispatchers|CreateEvent :!event EndOfLevel)))

(fn ConstructionScript)

(fn AddGold
  (params (amountToAdd :type Integer))
  (bind _output_get (Variables|Default|Setgold (+ amountToAdd (Variables|Default|Getgold))))
  (return _output_get))

(fn GetSurvivingUnits
  (bind _outactors (Actor|GetAllActorsOfClasswithTag "/Game/dungeon_assets/Units/BP_MasterU.BP_MasterU_C" "Friendly"))
  (bind _output_get (Variables|Default|Setunits _outactors))
  (return _output_get))

(fn EndOfLevel
  (bind _isvictory (CallFunction|CheckforVictory))
  (if _isvictory
    (CallFunction|RunVictoryCode)
    (Development|PrintString "Victory")
    (else
      (CallFunction|RunDefeatCode)
      (Development|PrintString "Defeat")))
  (EventDispatchers|UnbindallEventsfromEndOfLevelDispatcher))

(fn CheckforVictory
  (bind _units (CallFunction|GetSurvivingUnits))
  (return (> (Utilities|Array|Length _units) 0)))

(fn ConvertUnitstoGold
  (for _array_element (Variables|Default|Getunits)
    (CallFunction|AddGold (Variables|/Game/dungeon_assets/Units/BP_MasterU.BP_MasterU_C|Getcost _array_element))))

(fn IncrementLevel
  (Math|Integer|IncrementInt (Variables|Default|Getround)))

(fn RunVictoryCode
  (CallFunction|GetSurvivingUnits)
  (CallFunction|ConvertUnitstoGold)
  (CallFunction|IncrementLevel))

(fn RunDefeatCode)