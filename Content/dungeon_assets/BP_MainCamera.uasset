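; BP_MainCamera is a camera Blueprint that pans along the world X axis in response to player input.
; On BeginPlay it places its SpringArm at a fixed world position and rotation.
; The Vertical axis input then shifts the SpringArm forward or back along X by CameraSpeed per update, keeping other transform values.
; Movement depends only on the input's sign and is not scaled by delta time.
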(event EventBeginPlay
  (Transformation|SetWorldTransform (Variables|Default|GetSpringArm) (Math|Transform|MakeTransform "125.000000,1.000000,-125.000000" "0.000000,-90.000000,0.000000" "1.000000,1.000000,1.000000") false false))

(event Input|AxisEvents|InputAxisVertical
  (params (AxisValue :type Float%20%28single-precision%29))
  (bind _springarm (Variables|Default|GetSpringArm))
  (bind _springarm_2 (Variables|Default|GetSpringArm))
  (bind _returnvalue (Transformation|GetWorldLocation _springarm_2))
  (bind _returnvalue_2 (Transformation|GetWorldLocation _springarm))
  (if (> AxisValue 0.0)
    (Transformation|SetWorldTransform (Variables|Default|GetSpringArm) (Math|Transform|MakeTransform (Math|Vector|MakeVector (+ (.x _returnvalue_2) (Variables|Default|GetcameraSpeed)) (.y _returnvalue_2) (.z _returnvalue_2)) (Transformation|GetWorldRotation _springarm) (Transformation|GetWorldScale _springarm)) false false)
    (elif (< AxisValue 0.0)
      (Transformation|SetWorldTransform (Variables|Default|GetSpringArm) (Math|Transform|MakeTransform (Math|Vector|MakeVector (- (.x _returnvalue) (Variables|Default|GetcameraSpeed)) (.y _returnvalue) (.z _returnvalue)) (Transformation|GetWorldRotation _springarm_2) (Transformation|GetWorldScale _springarm_2)) false false))))

(fn ConstructionScript)