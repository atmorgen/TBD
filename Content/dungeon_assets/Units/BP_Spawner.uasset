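; BP_Spawner is a Blueprint that spawns units at a tagged location in the level.
; On BeginPlay it caches the first actor tagged "Spawn" as its spawn location, provided that actor is a PaperSpriteActor.
; SpawnUnit converts the requested unit to a row name in UnitDataTable and, when found, spawns that row's class at the sprite's render component world transform.
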(event EventBeginPlay
  (bind _outactors (Actor|GetAllActorswithTag "Spawn"))
  (bind _aspaper_sprite_actor (Utilities|Casting|CastToPaperSpriteActor (Utilities|Array|Get(acopy) _outactors)))
  (Variables|Default|SetspawnLocation _aspaper_sprite_actor))

(fn ConstructionScript)

(fn SpawnUnit
  (params (targetUnit :type String))
  (bind _returnvalue (Utilities|GetDataTableRow "/Game/dungeon_assets/Units/data/UnitDataTable.UnitDataTable" (Utilities|String|StringToName targetUnit))
    (:then
      (Game|SpawnActorfromClass (Utilities|Struct|BreakFUnitInfo _returnvalue) (Transformation|GetWorldTransform (Variables|/Script/Paper2D.PaperSpriteActor|GetRenderComponent (Variables|Default|GetspawnLocation))) "Undefined" 0 0))))