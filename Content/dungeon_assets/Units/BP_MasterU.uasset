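; Base Paper2D unit for automatic battles between actors tagged Friendly and Enemy, with stats loaded from a data table by unit name.
; Each Tick calls StartRound to find the nearest opponent, then moves toward it with a yaw-flipping sprite or attacks on a tick-incremented cooldown.
; Attacks subtract health directly and swap flipbooks; the healthbar update destroys depleted units.
; Without a valid target, the unit destroys itself and prints "Round Over".
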(event Custom|asdf
  ;[1 1 1] HOLDER STUFF FOR UNIT BEING DAMAGED.  Makes the UNIT RED FOR A SECOND
)

(event Custom|StartRound
  ;[1 1 1] NORMAN USE THIS AS START OF ROUND
  (bind _enemytarget (CallFunction|FindClosestEnemy))
  (if (Utilities|IsValid _enemytarget)
    (bind (_inrange _enemy) (CallFunction|InRangetoAttack _enemytarget))
    (if _inrange
      (CallFunction|AttackLogic)
      (else
        (CallFunction|MovetoClosestEnemy _enemy)
        (CallFunction|AnimateMovement)))
    (CallFunction|UpdateHealthbar)
    (else
      ;[1 1 1] THIS IS WHERE THE ROUND ENDS. DOES NOT DIFFERENTIATE BETWEEN GOOD/BAD WIN.  Probably should
      (CallFunction|EverythingIsDead))))

(event EventBeginPlay
  (CallFunction|SetStartingValues)
  (CallFunction|UpdateHealthbar)
  (CallFunction|DetermineIsFriendly))

(event EventTick
  (params (DeltaSeconds :type Float%20%28single-precision%29))
  ;[1 1 1] WE WILL GET RID OF THIS ONCE WE HAVE A BETTER START
  (CallFunction|StartRound))

(fn ConstructionScript)

(fn MovetoClosestEnemy
  (params (enemyTarget :type BP%20Master%20U%20Object%20Reference))
  (if (Utilities|IsValid enemyTarget)
    (Transformation|SetActorLocation (Math|Interpolation|VInterptoConstant (.location (Transformation|GetWorldTransform (Variables|Default|GetPaperFlipbook))) (.location (Transformation|GetWorldTransform (Variables|BP_MasterU_C|GetPaperFlipbook enemyTarget))) 1.0 (* (Variables|Default|Getspeed) (Utilities|Time|GetWorldDeltaSeconds))) false false)))

(fn UpdateHealthbar
  (bind _aswb_healthbar (Utilities|Casting|CastToWB_Healthbar (UserInterface|GetUserWidgetObject (Variables|Default|GetHealthbar))))
  (bind _output_get (Variables|/Game/dungeon_assets/Units/WB_Healthbar.WB_Healthbar_C|Sethealth _aswb_healthbar (/ (Variables|Default|GetcurrentHealth) (Variables|Default|GetmaxHealth))))
  (if (> _output_get 0.0)
    _
    (else
      (CallFunction|Death)))
  (return))

(fn DetermineIsFriendly
  (for _array_element (Variables|Actor|GetTags self)
    (switch name _array_element
      (:Friendly
        (Variables|Default|SetisFriendly true))
      (:Enemy
        (Variables|Default|SetisFriendly false)))))

(fn FindClosestEnemy
  (bind _paperflipbook (Variables|Default|GetPaperFlipbook))
  (bind _returnvalue (Transformation|GetWorldLocation _paperflipbook))
  (if (Variables|Default|GetisFriendly)
    (bind _outactors (Actor|GetAllActorswithTag "Enemy"))
    (bind _asbp_master_u (Utilities|Casting|CastToBP_MasterU (.ReturnValue (Actor|FindNearestActor _returnvalue _outactors))))
    (bind _output_get (Variables|Default|Settarget _asbp_master_u))
    (return _output_get)
    (else
      (bind _outactors_2 (Actor|GetAllActorswithTag "Friendly"))
      (bind _asbp_master_u_2 (Utilities|Casting|CastToBP_MasterU (.ReturnValue (Actor|FindNearestActor _returnvalue _outactors_2))))
      (bind _output_get_2 (Variables|Default|Settarget _asbp_master_u_2))
      (return _output_get_2))))

(fn InRangetoAttack
  (params (enemyTarget :type BP%20Master%20U%20Object%20Reference))
  (bind _output_get (Variables|Default|SetinAttackRange (<= (Math|Vector|VectorLength (- (Transformation|GetWorldLocation (Variables|BP_MasterU_C|GetPaperFlipbook enemyTarget)) (Transformation|GetWorldLocation (Variables|Default|GetPaperFlipbook)))) (Variables|Default|GetattackRange))))
  (return _output_get enemyTarget))

(fn AttackTarget
  (params (enemyTarget :type BP%20Master%20U%20Object%20Reference))
  (Utilities|Time|SetTimerbyFunctionName 0 "death" (Variables|Default|GetattackSpeed) true)
  (return))

(fn AnimateAttack
  (Sprite|SetFlipbook (Variables|Default|GetPaperFlipbook) (Variables|Default|Getattack_flipbook)))

(fn AnimateMovement
  (Sprite|SetFlipbook (Variables|Default|GetPaperFlipbook) (Variables|Default|Getmovement_flipbook))
  (CallFunction|LerpRotate))

(fn Death
  (Actor|DestroyActor self))

(fn EverythingIsDead
  (Actor|DestroyActor)
  (Development|PrintText "Round Over"))

(fn AttackLogic
  (bind _canattack (CallFunction|CanAttack))
  (if _canattack
    (CallFunction|DamageTarget)
    (Rendering|Debug|DrawDebugLine (Transformation|GetWorldLocation (Variables|Default|GetPaperFlipbook)) (Transformation|GetWorldLocation (Variables|BP_MasterU_C|GetPaperFlipbook (Variables|Default|Gettarget))) (Class|KismetMathLibrary|LinearColorRed) 0.1 0.5)
    (CallFunction|AnimateAttack)
    (CallFunction|WasHit (Variables|Default|Gettarget))))

(fn DamageTarget
  (Variables|BP_MasterU_C|SetcurrentHealth (Variables|Default|Gettarget) (- (Variables|BP_MasterU_C|GetcurrentHealth (Variables|Default|Gettarget)) (Variables|Default|Getdamage))))

(fn CanAttack
  (if (>= (Variables|Default|GetattackTimer) (Variables|Default|GetattackSpeed))
    (Variables|Default|SetattackTimer 0.0)
    (return true)
    (else
      (Variables|Default|SetattackTimer (+ (Variables|Default|GetattackTimer) 0.1)))))

(fn WasHit
  (bind _paperflipbook (Variables|Default|GetPaperFlipbook))
  (if (<= (Variables|Default|GetcurrentHealth) 0.0)
    (Sprite|SetFlipbook _paperflipbook (Variables|Default|Getdeath_flipbook))
    (else
      (Sprite|SetFlipbook _paperflipbook (Variables|Default|Getdamaged_flipbook)))))

(fn SetStartingValues
  (bind _returnvalue (Utilities|GetDataTableRow "/Game/dungeon_assets/Units/data/UnitDataTable.UnitDataTable" (Utilities|String|StringToName (Variables|Default|GetunitName)))
    (:then
      (Variables|Default|SetmaxHealth (.MaxHealth (Utilities|Struct|BreakFUnitInfo _returnvalue)))
      (Variables|Default|SetcurrentHealth (.MaxHealth (Utilities|Struct|BreakFUnitInfo _returnvalue)))
      (Variables|Default|Setspeed (.Speed (Utilities|Struct|BreakFUnitInfo _returnvalue)))
      (Variables|Default|Setdamage (.Damage (Utilities|Struct|BreakFUnitInfo _returnvalue)))
      (Variables|Default|SetattackSpeed (.AttackSpeed (Utilities|Struct|BreakFUnitInfo _returnvalue)))
      (Variables|Default|SetattackRange (.AttackRange (Utilities|Struct|BreakFUnitInfo _returnvalue))))))

(fn LerpRotate
  ;[1 1 1] Logic make the sprites flip based on location of the target.  This should probably go in it's own class...
  (if (>= (.x (Transformation|GetWorldLocation (Variables|/Script/Paper2D.PaperSpriteActor|GetRenderComponent (Variables|Default|Gettarget)))) (.x (Transformation|GetWorldLocation (Variables|Default|GetRenderComponent))))
    (if (>= (Variables|Default|GetlerpRotValue) 0.0)
      (Variables|Default|SetlerpRotValue (- (Variables|Default|GetlerpRotValue) 4.0))
      (Transformation|SetWorldRotation (Variables|Default|GetPaperFlipbook) (Math|Rotator|MakeRotator 0.0 0.0 (Variables|Default|GetlerpRotValue)) false false :!label _label))
    (elif (<= (Variables|Default|GetlerpRotValue) 1.8e+02)
      (Variables|Default|SetlerpRotValue (+ (Variables|Default|GetlerpRotValue) 4.0))
      (goto _label))))