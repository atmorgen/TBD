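; Necromancer unit Blueprint with a test beam-style attack bound directly to the 1 key.
; Pressing the key restarts a timeline whose track sets the length of a debug-drawn box trace along the render component's forward vector, on the Camera channel.
; Each update subtracts a fixed amount of CurrentHealth from any BP_MasterU hit, so damage depends on frame rate.
; Releasing the key stops the timeline.
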(event EventBeginPlay
  (|CallParentFunction))

(event Collision|EventActorBeginOverlap
  (params (OtherActor :type Actor%20Object%20Reference)))

(event EventTick
  (params (DeltaSeconds :type Float%20%28single-precision%29))
  (|CallParentFunction DeltaSeconds))

(event Input|KeyboardEvents|1
  (params (Key :type Key%20Structure :default "None"))
  (bind _self self)
  (bind _rendercomponent (Variables|Default|GetRenderComponent _self))
  (bind _returnvalue (Transformation|GetWorldLocation _rendercomponent))
  (:Pressed
    (bind _newtrack_0 (Timeline|Timeline PlayFromStart)
      (:Update
        (bind _output_get (Variables|Default|SettestLength _newtrack_0))
        (bind _outhit (Collision|BoxTraceByChannel _returnvalue (+ _returnvalue (* (Math|Vector|GetForwardVector (Variables|Default|GetRenderComponent _self)) _output_get)) "7.500000,5.000000,7.500000" "0, 0, 0" "TraceTypeQuery2" false 0 "ForDuration" true "(R=1.000000,G=0.000000,B=0.000000,A=1.000000)" "(R=0.000000,G=1.000000,B=0.000000,A=1.000000)" 0.2))
        (bind _asbp_master_u (Utilities|Casting|CastToBP_MasterU (.HitActor (Collision|BreakHitResult _outhit))))
        (Variables|/Game/dungeon_assets/Units/BP_MasterU.BP_MasterU_C|SetcurrentHealth _asbp_master_u (- (Variables|/Game/dungeon_assets/Units/BP_MasterU.BP_MasterU_C|GetcurrentHealth _asbp_master_u) 0.1)))))
  (:Released
    (Timeline|Timeline Stop)))

(fn ConstructionScript
  (|CallParentFunction))